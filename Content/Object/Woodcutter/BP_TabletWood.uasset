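; Woodcutter upgrade tablet that lets the player spend wood and stone to advance through two levels.
; Tick writes the current level's cost and prompt text to the third-person character's TabletW variables.
; Interacting via BPC_InteractableObject checks inventory, deducts resources and sets Lvl1 or Lvl2, or briefly shows a LowResurse widget.
; At max level, interaction sets TabletMineText instead of TabletWText.
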(event OnInterected(BPC_InteractableObject)
  (bind _as_bp_third_person_character (Variables|Default|GetAs%20BP%20Third%20Person%20Character))
  (bind _as_bp_third_person_character_2 (Variables|Default|GetAs%20BP%20Third%20Person%20Character))
  (bind _as_bp_third_person_character_3 (Variables|Default|GetAs%20BP%20Third%20Person%20Character))
  (if (Variables|Default|GetLvl1)
    (if (>= (Variables|/Game/Widget/WB_Inventory.WB_Inventory_C|GetIntWood (Variables|/Game/ThirdPerson/Blueprints/BP_ThirdPersonCharacter.BP_ThirdPersonCharacter_C|GetInventory (Variables|Default|GetAs%20BP%20Third%20Person%20Character))) 10)
      (if (>= (Variables|/Game/Widget/WB_Inventory.WB_Inventory_C|GetIntStone (Variables|/Game/ThirdPerson/Blueprints/BP_ThirdPersonCharacter.BP_ThirdPersonCharacter_C|GetInventory (Variables|Default|GetAs%20BP%20Third%20Person%20Character))) 10)
        (Default|MinusStone _as_bp_third_person_character_3 10)
        (Default|MinusWood _as_bp_third_person_character_3 10)
        (Variables|Default|SetLvl2 true)
        (Variables|Default|SetLvl1 false)
        (else
          (Widget|RemovefromParent (Variables|Default|GetLow))
          (bind _returnvalue (UserInterface|CreateWidget "/Game/Widget/LowResurse.LowResurse_C"))
          (UserInterface|Viewport|AddtoViewport _returnvalue 0)
          (Utilities|FlowControl|Delay 2.0)
          (Widget|RemovefromParent _returnvalue)))
      (else
        (Widget|RemovefromParent (Variables|Default|GetLow))
        (bind _returnvalue_2 (UserInterface|CreateWidget "/Game/Widget/LowResurse.LowResurse_C"))
        (UserInterface|Viewport|AddtoViewport _returnvalue_2 0)
        (Utilities|FlowControl|Delay 2.0)
        (Widget|RemovefromParent _returnvalue_2)))
    (elif (Variables|Default|GetLvl2)
      (Default|MinusStone _as_bp_third_person_character)
      (Default|MinusWood _as_bp_third_person_character)
      (Variables|/Game/ThirdPerson/Blueprints/BP_ThirdPersonCharacter.BP_ThirdPersonCharacter_C|SetTabletMineText _as_bp_third_person_character "Максимальный уровень")
      (elif (>= (Variables|/Game/Widget/WB_Inventory.WB_Inventory_C|GetIntWood (Variables|/Game/ThirdPerson/Blueprints/BP_ThirdPersonCharacter.BP_ThirdPersonCharacter_C|GetInventory (Variables|Default|GetAs%20BP%20Third%20Person%20Character))) 5)
        (if (>= (Variables|/Game/Widget/WB_Inventory.WB_Inventory_C|GetIntStone (Variables|/Game/ThirdPerson/Blueprints/BP_ThirdPersonCharacter.BP_ThirdPersonCharacter_C|GetInventory (Variables|Default|GetAs%20BP%20Third%20Person%20Character))) 5)
          (Default|MinusStone _as_bp_third_person_character_2 5)
          (Default|MinusWood _as_bp_third_person_character_2 5)
          (Variables|Default|SetLvl1 true)
          (else
            (Widget|RemovefromParent (Variables|Default|GetLow))
            (bind _returnvalue_3 (UserInterface|CreateWidget "/Game/Widget/LowResurse.LowResurse_C"))
            (UserInterface|Viewport|AddtoViewport _returnvalue_3 0)
            (Utilities|FlowControl|Delay 2.0)
            (Widget|RemovefromParent _returnvalue_3)))
        (else
          (Widget|RemovefromParent (Variables|Default|GetLow))
          (bind _returnvalue_4 (UserInterface|CreateWidget "/Game/Widget/LowResurse.LowResurse_C"))
          (bind _output_get (Variables|Default|SetLow _returnvalue_4))
          (UserInterface|Viewport|AddtoViewport _output_get 0)
          (Utilities|FlowControl|Delay 2.0)
          (Widget|RemovefromParent _output_get))))))

(event EventBeginPlay
  (bind _asbp_third_person_character (Utilities|Casting|CastToBP_ThirdPersonCharacter (Game|Player|GetPlayerPawn 0)))
  (Variables|Default|SetAs%20BP%20Third%20Person%20Character _asbp_third_person_character))

(event Collision|EventActorBeginOverlap
  (params (OtherActor :type Actor%20Object%20Reference)))

(event EventTick
  (params (DeltaSeconds :type Float%20%28single-precision%29))
  (bind _as_bp_third_person_character (Variables|Default|GetAs%20BP%20Third%20Person%20Character))
  (bind _as_bp_third_person_character_2 (Variables|Default|GetAs%20BP%20Third%20Person%20Character))
  (bind _as_bp_third_person_character_3 (Variables|Default|GetAs%20BP%20Third%20Person%20Character))
  (if (Variables|Default|GetLvl1)
    (Variables|/Game/ThirdPerson/Blueprints/BP_ThirdPersonCharacter.BP_ThirdPersonCharacter_C|SetTabletWStone _as_bp_third_person_character_3 10)
    (Variables|/Game/ThirdPerson/Blueprints/BP_ThirdPersonCharacter.BP_ThirdPersonCharacter_C|SetTabletWWood _as_bp_third_person_character_3 10)
    (Variables|/Game/ThirdPerson/Blueprints/BP_ThirdPersonCharacter.BP_ThirdPersonCharacter_C|SetTabletWText _as_bp_third_person_character_3 "Улучшить?")
    (elif (Variables|Default|GetLvl2)
      (Variables|/Game/ThirdPerson/Blueprints/BP_ThirdPersonCharacter.BP_ThirdPersonCharacter_C|SetTabletWStone _as_bp_third_person_character_2 0)
      (Variables|/Game/ThirdPerson/Blueprints/BP_ThirdPersonCharacter.BP_ThirdPersonCharacter_C|SetTabletWWood _as_bp_third_person_character_2 0)
      (Variables|/Game/ThirdPerson/Blueprints/BP_ThirdPersonCharacter.BP_ThirdPersonCharacter_C|SetTabletWText _as_bp_third_person_character_2 "Максимальный уровень!")
      (else
        (Variables|/Game/ThirdPerson/Blueprints/BP_ThirdPersonCharacter.BP_ThirdPersonCharacter_C|SetTabletWStone _as_bp_third_person_character 5)
        (Variables|/Game/ThirdPerson/Blueprints/BP_ThirdPersonCharacter.BP_ThirdPersonCharacter_C|SetTabletWWood _as_bp_third_person_character 5)
        (Variables|/Game/ThirdPerson/Blueprints/BP_ThirdPersonCharacter.BP_ThirdPersonCharacter_C|SetTabletWText _as_bp_third_person_character "Улучшить?")))))

(fn ConstructionScript)