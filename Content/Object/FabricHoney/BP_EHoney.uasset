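; BP_EHoney is an interactable object that trades the player's Fabric for EHoney.
; It caches the player's BP_ThirdPersonCharacter on BeginPlay.
; When its BPC_InteractableObject component reports an interaction while the referenced Object's InputOn flag is set, it adds one EHoney, clears the flag and removes one Fabric.
; The Blueprint itself does no check on the player's Fabric count.
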(event OnInterected(BPC_InteractableObject)
  (bind _as_bp_third_person_character (Variables|Default|GetAs%20BP%20Third%20Person%20Character))
  (if (Variables|/Game/Object/FabricHoney/BP_Honey.BP_Honey_C|GetInputOn (Variables|Default|GetObject))
    (Default|AddEHoney _as_bp_third_person_character 1)
    (Variables|/Game/Object/FabricHoney/BP_Honey.BP_Honey_C|SetInputOn (Variables|Default|GetObject) false)
    (Default|MinusFabric _as_bp_third_person_character 1)))

(event EventBeginPlay
  (bind _asbp_third_person_character (Utilities|Casting|CastToBP_ThirdPersonCharacter (Game|Player|GetPlayerPawn 0)))
  (Variables|Default|SetAs%20BP%20Third%20Person%20Character _asbp_third_person_character))

(event Collision|EventActorBeginOverlap
  (params (OtherActor :type Actor%20Object%20Reference)))

(event EventTick
  (params (DeltaSeconds :type Float%20%28single-precision%29)))

(fn ConstructionScript)