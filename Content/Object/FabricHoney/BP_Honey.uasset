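; BP_Honey is an interactable actor that trades one honey from the player's inventory for one fabric.
; On interaction it checks the third-person character cached at BeginPlay, then calls its MinusHoney and AddFabric functions.
; The InputOn flag is never reset here, so the trade succeeds only once.
; Without enough honey it shows a LowResurse widget for two seconds, with the Upgrade flag blocking duplicate popups.
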(event OnInterected(BPC_InteractableObject)
  (bind _as_bp_third_person_character (Variables|Default|GetAs%20BP%20Third%20Person%20Character))
  (if (not (Variables|Default|GetInputOn))
    (if (>= (Variables|/Game/Widget/WB_Inventory.WB_Inventory_C|GetIntHoney (Variables|/Game/ThirdPerson/Blueprints/BP_ThirdPersonCharacter.BP_ThirdPersonCharacter_C|GetInventory (Variables|Default|GetAs%20BP%20Third%20Person%20Character))) 1)
      (Default|MinusHoney _as_bp_third_person_character 1)
      (Variables|Default|SetInputOn true)
      (Default|AddFabric _as_bp_third_person_character 1)
      (elif (not (Variables|Default|GetUpgrade))
        (bind _returnvalue (UserInterface|CreateWidget "/Game/Widget/LowResurse.LowResurse_C"))
        (UserInterface|Viewport|AddtoViewport _returnvalue 0)
        (Variables|Default|SetUpgrade true)
        (Utilities|FlowControl|Delay 2.0)
        (Widget|RemovefromParent _returnvalue)
        (Variables|Default|SetUpgrade false)))))

(event EventBeginPlay
  (bind _asbp_third_person_character (Utilities|Casting|CastToBP_ThirdPersonCharacter (Game|Player|GetPlayerPawn 0)))
  (Variables|Default|SetAs%20BP%20Third%20Person%20Character _asbp_third_person_character))

(event Collision|EventActorBeginOverlap
  (params (OtherActor :type Actor%20Object%20Reference)))

(event EventTick
  (params (DeltaSeconds :type Float%20%28single-precision%29)))

(fn ConstructionScript)