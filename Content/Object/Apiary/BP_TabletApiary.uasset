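; Interactable apiary tablet that lets the player buy two upgrade levels with inventory resources.
; Tick writes the next level's wood, iron and honey cost and the prompt or max-level text to the cached player character.
; On interaction it checks the inventory, deducts the cost and advances the Lvl1/Lvl2 flags.
; A shortfall briefly shows the LowResurse widget, with the Upgrade flag blocking duplicate warnings.
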(event OnInterected(BPC_InteractableObject)
  (bind _as_bp_third_person_character (Variables|Default|GetAs%20BP%20Third%20Person%20Character))
  (bind _as_bp_third_person_character_2 (Variables|Default|GetAs%20BP%20Third%20Person%20Character))
  (if (Variables|Default|GetLvl1)
    (if (>= (Variables|/Game/Widget/WB_Inventory.WB_Inventory_C|GetIntWood (Variables|/Game/ThirdPerson/Blueprints/BP_ThirdPersonCharacter.BP_ThirdPersonCharacter_C|GetInventory (Variables|Default|GetAs%20BP%20Third%20Person%20Character))) 10)
      (if (>= (Variables|/Game/Widget/WB_Inventory.WB_Inventory_C|GetIntIron (Variables|/Game/ThirdPerson/Blueprints/BP_ThirdPersonCharacter.BP_ThirdPersonCharacter_C|GetInventory (Variables|Default|GetAs%20BP%20Third%20Person%20Character))) 10)
        (if (>= (Variables|/Game/Widget/WB_Inventory.WB_Inventory_C|GetIntHoney (Variables|/Game/ThirdPerson/Blueprints/BP_ThirdPersonCharacter.BP_ThirdPersonCharacter_C|GetInventory (Variables|Default|GetAs%20BP%20Third%20Person%20Character))) 5)
          (Default|MinusIron _as_bp_third_person_character_2 10)
          (Default|MinusWood _as_bp_third_person_character_2 10)
          (Default|MinusHoney _as_bp_third_person_character_2 5)
          (Variables|Default|SetLvl1 false)
          (Variables|Default|SetLvl2 true)
          (elif (not (Variables|Default|GetUpgrade))
            (bind _returnvalue (UserInterface|CreateWidget "/Game/Widget/LowResurse.LowResurse_C"))
            (UserInterface|Viewport|AddtoViewport _returnvalue 0)
            (Variables|Default|SetUpgrade true)
            (Utilities|FlowControl|Delay 2.0)
            (Widget|RemovefromParent _returnvalue)
            (Variables|Default|SetUpgrade false)))
        (elif (not (Variables|Default|GetUpgrade))
          (bind _returnvalue_2 (UserInterface|CreateWidget "/Game/Widget/LowResurse.LowResurse_C"))
          (UserInterface|Viewport|AddtoViewport _returnvalue_2 0)
          (Variables|Default|SetUpgrade true)
          (Utilities|FlowControl|Delay 2.0)
          (Widget|RemovefromParent _returnvalue_2)
          (Variables|Default|SetUpgrade false)))
      (elif (not (Variables|Default|GetUpgrade))
        (bind _returnvalue_3 (UserInterface|CreateWidget "/Game/Widget/LowResurse.LowResurse_C"))
        (UserInterface|Viewport|AddtoViewport _returnvalue_3 0)
        (Variables|Default|SetUpgrade true)
        (Utilities|FlowControl|Delay 2.0)
        (Widget|RemovefromParent _returnvalue_3)
        (Variables|Default|SetUpgrade false)))
    (elif (not (Variables|Default|GetLvl2))
      (if (>= (Variables|/Game/Widget/WB_Inventory.WB_Inventory_C|GetIntWood (Variables|/Game/ThirdPerson/Blueprints/BP_ThirdPersonCharacter.BP_ThirdPersonCharacter_C|GetInventory (Variables|Default|GetAs%20BP%20Third%20Person%20Character))) 5)
        (if (>= (Variables|/Game/Widget/WB_Inventory.WB_Inventory_C|GetIntIron (Variables|/Game/ThirdPerson/Blueprints/BP_ThirdPersonCharacter.BP_ThirdPersonCharacter_C|GetInventory (Variables|Default|GetAs%20BP%20Third%20Person%20Character))) 5)
          (Default|MinusIron _as_bp_third_person_character 5)
          (Default|MinusWood _as_bp_third_person_character 5)
          (Variables|Default|SetLvl1 true)
          (elif (not (Variables|Default|GetUpgrade))
            (bind _returnvalue_4 (UserInterface|CreateWidget "/Game/Widget/LowResurse.LowResurse_C"))
            (UserInterface|Viewport|AddtoViewport _returnvalue_4 0)
            (Variables|Default|SetUpgrade true)
            (Utilities|FlowControl|Delay 2.0)
            (Widget|RemovefromParent _returnvalue_4)
            (Variables|Default|SetUpgrade false)))
        (elif (not (Variables|Default|GetUpgrade))
          (bind _returnvalue_5 (UserInterface|CreateWidget "/Game/Widget/LowResurse.LowResurse_C"))
          (UserInterface|Viewport|AddtoViewport _returnvalue_5 0)
          (Variables|Default|SetUpgrade true)
          (Utilities|FlowControl|Delay 2.0)
          (Widget|RemovefromParent _returnvalue_5)
          (Variables|Default|SetUpgrade false))))))

(event EventBeginPlay
  (bind _asbp_third_person_character (Utilities|Casting|CastToBP_ThirdPersonCharacter (Game|Player|GetPlayerPawn 0)))
  (Variables|Default|SetAs%20BP%20Third%20Person%20Character _asbp_third_person_character))

(event Collision|EventActorBeginOverlap
  (params (OtherActor :type Actor%20Object%20Reference)))

(event EventTick
  (params (DeltaSeconds :type Float%20%28single-precision%29))
  (bind _as_bp_third_person_character (Variables|Default|GetAs%20BP%20Third%20Person%20Character))
  (bind _as_bp_third_person_character_2 (Variables|Default|GetAs%20BP%20Third%20Person%20Character))
  (bind _as_bp_third_person_character_3 (Variables|Default|GetAs%20BP%20Third%20Person%20Character))
  (if (Variables|Default|GetLvl1)
    (Variables|/Game/ThirdPerson/Blueprints/BP_ThirdPersonCharacter.BP_ThirdPersonCharacter_C|SetApiaryWood _as_bp_third_person_character 10)
    (Variables|/Game/ThirdPerson/Blueprints/BP_ThirdPersonCharacter.BP_ThirdPersonCharacter_C|SetApiaryIron _as_bp_third_person_character 10)
    (Variables|/Game/ThirdPerson/Blueprints/BP_ThirdPersonCharacter.BP_ThirdPersonCharacter_C|SetApiaryHoney _as_bp_third_person_character 5)
    (Variables|/Game/ThirdPerson/Blueprints/BP_ThirdPersonCharacter.BP_ThirdPersonCharacter_C|SetTabletMineText _as_bp_third_person_character "Улучшить?")
    (elif (Variables|Default|GetLvl2)
      (Variables|/Game/ThirdPerson/Blueprints/BP_ThirdPersonCharacter.BP_ThirdPersonCharacter_C|SetApiaryWood _as_bp_third_person_character_3 0)
      (Variables|/Game/ThirdPerson/Blueprints/BP_ThirdPersonCharacter.BP_ThirdPersonCharacter_C|SetApiaryIron _as_bp_third_person_character_3 0)
      (Variables|/Game/ThirdPerson/Blueprints/BP_ThirdPersonCharacter.BP_ThirdPersonCharacter_C|SetApiaryHoney _as_bp_third_person_character_3 0)
      (Variables|/Game/ThirdPerson/Blueprints/BP_ThirdPersonCharacter.BP_ThirdPersonCharacter_C|SetTabletMineText _as_bp_third_person_character_3 "Максимальный уровень!")
      (else
        (Variables|/Game/ThirdPerson/Blueprints/BP_ThirdPersonCharacter.BP_ThirdPersonCharacter_C|SetApiaryWood _as_bp_third_person_character_2 5)
        (Variables|/Game/ThirdPerson/Blueprints/BP_ThirdPersonCharacter.BP_ThirdPersonCharacter_C|SetApiaryIron _as_bp_third_person_character_2 5)
        (Variables|/Game/ThirdPerson/Blueprints/BP_ThirdPersonCharacter.BP_ThirdPersonCharacter_C|SetApiaryHoney _as_bp_third_person_character_2 0)
        (Variables|/Game/ThirdPerson/Blueprints/BP_ThirdPersonCharacter.BP_ThirdPersonCharacter_C|SetTabletMineText _as_bp_third_person_character_2 "Улучшить?")))))

(fn ConstructionScript)