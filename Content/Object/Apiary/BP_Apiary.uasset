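; BP_Apiary is an interactable apiary that passively produces honey for the player's BP_ThirdPersonCharacter.
; A Passive event re-arms its own looping timer, adding one apiary honey to the character per call via AddApiHoney.
; The Tablet's Lvl1 and Lvl2 flags set the interval used when the timer is next re-armed.
; Interacting through BPC_InteractableObject passes the character's Honey value to AddHoney, then zeroes it.
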(event OnInterected(BPC_InteractableObject)
  (bind _qwer (Variables|Default|Getqwer))
  (Default|AddHoney _qwer (Variables|/Game/ThirdPerson/Blueprints/BP_ThirdPersonCharacter.BP_ThirdPersonCharacter_C|GetHoney _qwer))
  (Variables|/Game/ThirdPerson/Blueprints/BP_ThirdPersonCharacter.BP_ThirdPersonCharacter_C|SetHoney _qwer 0))

(event Custom|Passive
  (Utilities|Time|SetTimerbyEvent (delegate Custom|Passive) (Variables|Default|GetTime_0) true)
  (if (Variables|/Game/Object/Apiary/BP_TabletApiary.BP_TabletApiary_C|GetLvl1 (Variables|Default|GetTablet))
    (Default|AddApiHoney (Variables|Default|Getqwer) 1)
    (Variables|Default|SetTime_0 5.0)
    (elif (Variables|/Game/Object/Apiary/BP_TabletApiary.BP_TabletApiary_C|GetLvl2 (Variables|Default|GetTablet))
      (Default|AddApiHoney (Variables|Default|Getqwer) 1)
      (Variables|Default|SetTime_0 2.5)
      (else
        (Default|AddApiHoney (Variables|Default|Getqwer) 1)
        (Variables|Default|SetTime_0 7.5)))))

(event EventBeginPlay
  (bind _asbp_third_person_character (Utilities|Casting|CastToBP_ThirdPersonCharacter (Game|Player|GetPlayerPawn 0)))
  (Variables|Default|Setqwer _asbp_third_person_character)
  (CallFunction|Passive))

(event Collision|EventActorBeginOverlap
  (params (OtherActor :type Actor%20Object%20Reference)))

(event EventTick
  (params (DeltaSeconds :type Float%20%28single-precision%29)))

(fn ConstructionScript)