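; Mine object that passively produces stone and iron, which the player collects by interacting with it.
; A self-rearming timer event adds to mine counters stored on the player character, with Tablet level flags enabling iron and shorter intervals.
; Lvl1 is checked before Lvl2, and each new interval is set after the timer is armed.
; Interaction through BPC_InteractableObject transfers the stored amounts to the player's totals and zeroes the counters.
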(event OnInterected(BPC_InteractableObject)
  (bind _qwer (Variables|Default|Getqwer))
  (Default|AddStone _qwer (Variables|/Game/ThirdPerson/Blueprints/BP_ThirdPersonCharacter.BP_ThirdPersonCharacter_C|GetMineStone _qwer))
  (Default|AddIron _qwer (Variables|/Game/ThirdPerson/Blueprints/BP_ThirdPersonCharacter.BP_ThirdPersonCharacter_C|GetMineIron _qwer))
  (Variables|/Game/ThirdPerson/Blueprints/BP_ThirdPersonCharacter.BP_ThirdPersonCharacter_C|SetMineStone _qwer 0)
  (Variables|/Game/ThirdPerson/Blueprints/BP_ThirdPersonCharacter.BP_ThirdPersonCharacter_C|SetMineIron _qwer 0))

(event Custom|Passive
  (bind _qwer (Variables|Default|Getqwer))
  (bind _qwer_2 (Variables|Default|Getqwer))
  (Utilities|Time|SetTimerbyEvent (delegate Custom|Passive) (Variables|Default|GetTime) true)
  (if (Variables|/Game/Object/Stone/BP_TabletMine.BP_TabletMine_C|GetLvl1 (Variables|Default|GetTablet))
    (Default|AddMineIron _qwer 1)
    (Default|AddMineStone _qwer 1)
    (Variables|Default|SetTime 5.0)
    (elif (Variables|/Game/Object/Stone/BP_TabletMine.BP_TabletMine_C|GetLvl2 (Variables|Default|GetTablet))
      (Default|AddMineIron _qwer_2 1)
      (Default|AddMineStone _qwer_2 1)
      (Variables|Default|SetTime 2.5)
      (else
        (Default|AddMineStone (Variables|Default|Getqwer) 1)
        (Variables|Default|SetTime 7.5)))))

(event EventBeginPlay
  (bind _asbp_third_person_character (Utilities|Casting|CastToBP_ThirdPersonCharacter (Game|Player|GetPlayerPawn 0)))
  (Variables|Default|Setqwer _asbp_third_person_character)
  (CallFunction|Passive))

(event Collision|EventActorBeginOverlap
  (params (OtherActor :type Actor%20Object%20Reference)))

(event EventTick
  (params (DeltaSeconds :type Float%20%28single-precision%29)))

(fn ConstructionScript)