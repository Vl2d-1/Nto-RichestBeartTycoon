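; Interactable tablet for a one-time portal upgrade paid with wood, stone, iron and E-honey from the player's inventory.
; Tick writes the costs and prompt text to the player character, switching to zero costs and a max-level message once upgraded.
; Interaction checks each resource, then deducts them and sets Lvl1, or briefly shows a LowResurse widget.
; The stone and iron check thresholds are swapped relative to the displayed and deducted costs.
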(event OnInterected(BPC_InteractableObject)
  (bind _as_bp_third_person_character (Variables|Default|GetAs%20BP%20Third%20Person%20Character))
  (if (not (Variables|Default|GetLvl1))
    (if (>= (Variables|/Game/Widget/WB_Inventory.WB_Inventory_C|GetIntWood (Variables|/Game/ThirdPerson/Blueprints/BP_ThirdPersonCharacter.BP_ThirdPersonCharacter_C|GetInventory (Variables|Default|GetAs%20BP%20Third%20Person%20Character))) 15)
      (if (>= (Variables|/Game/Widget/WB_Inventory.WB_Inventory_C|GetIntIron (Variables|/Game/ThirdPerson/Blueprints/BP_ThirdPersonCharacter.BP_ThirdPersonCharacter_C|GetInventory (Variables|Default|GetAs%20BP%20Third%20Person%20Character))) 15)
        (if (>= (Variables|/Game/Widget/WB_Inventory.WB_Inventory_C|GetIntStone (Variables|/Game/ThirdPerson/Blueprints/BP_ThirdPersonCharacter.BP_ThirdPersonCharacter_C|GetInventory (Variables|Default|GetAs%20BP%20Third%20Person%20Character))) 10)
          (if (>= (Variables|/Game/Widget/WB_Inventory.WB_Inventory_C|GetIntEHoney (Variables|/Game/ThirdPerson/Blueprints/BP_ThirdPersonCharacter.BP_ThirdPersonCharacter_C|GetInventory (Variables|Default|GetAs%20BP%20Third%20Person%20Character))) 5)
            (Default|MinusWood _as_bp_third_person_character 15)
            (Default|MinusStone _as_bp_third_person_character 15)
            (Default|MinusIron _as_bp_third_person_character 10)
            (Default|MinusEHoney _as_bp_third_person_character 5)
            (Variables|Default|SetLvl1 true)
            (else
              (Widget|RemovefromParent (Variables|Default|GetLow))
              (bind _returnvalue (UserInterface|CreateWidget "/Game/Widget/LowResurse.LowResurse_C"))
              (bind _output_get (Variables|Default|SetLow _returnvalue))
              (UserInterface|Viewport|AddtoViewport _output_get 0)
              (Utilities|FlowControl|Delay 2.0)
              (Widget|RemovefromParent _output_get)))
          (else
            (Widget|RemovefromParent (Variables|Default|GetLow))
            (bind _returnvalue_2 (UserInterface|CreateWidget "/Game/Widget/LowResurse.LowResurse_C"))
            (bind _output_get_2 (Variables|Default|SetLow _returnvalue_2))
            (UserInterface|Viewport|AddtoViewport _output_get_2 0)
            (Utilities|FlowControl|Delay 2.0)
            (Widget|RemovefromParent _output_get_2)))
        (else
          (Widget|RemovefromParent (Variables|Default|GetLow))
          (bind _returnvalue_3 (UserInterface|CreateWidget "/Game/Widget/LowResurse.LowResurse_C"))
          (bind _output_get_3 (Variables|Default|SetLow _returnvalue_3))
          (UserInterface|Viewport|AddtoViewport _output_get_3 0)
          (Utilities|FlowControl|Delay 2.0)
          (Widget|RemovefromParent _output_get_3)))
      (else
        (Widget|RemovefromParent (Variables|Default|GetLow))
        (bind _returnvalue_4 (UserInterface|CreateWidget "/Game/Widget/LowResurse.LowResurse_C"))
        (bind _output_get_4 (Variables|Default|SetLow _returnvalue_4))
        (UserInterface|Viewport|AddtoViewport _output_get_4 0)
        (Utilities|FlowControl|Delay 2.0)
        (Widget|RemovefromParent _output_get_4)))))

(event EventBeginPlay
  (bind _asbp_third_person_character (Utilities|Casting|CastToBP_ThirdPersonCharacter (Game|Player|GetPlayerPawn 0)))
  (Variables|Default|SetAs%20BP%20Third%20Person%20Character _asbp_third_person_character))

(event Collision|EventActorBeginOverlap
  (params (OtherActor :type Actor%20Object%20Reference)))

(event EventTick
  (params (DeltaSeconds :type Float%20%28single-precision%29))
  (bind _as_bp_third_person_character (Variables|Default|GetAs%20BP%20Third%20Person%20Character))
  (bind _as_bp_third_person_character_2 (Variables|Default|GetAs%20BP%20Third%20Person%20Character))
  (if (Variables|Default|GetLvl1)
    (Variables|/Game/ThirdPerson/Blueprints/BP_ThirdPersonCharacter.BP_ThirdPersonCharacter_C|SetPortalStone _as_bp_third_person_character_2 0)
    (Variables|/Game/ThirdPerson/Blueprints/BP_ThirdPersonCharacter.BP_ThirdPersonCharacter_C|SetPortalWood _as_bp_third_person_character_2 0)
    (Variables|/Game/ThirdPerson/Blueprints/BP_ThirdPersonCharacter.BP_ThirdPersonCharacter_C|SetPortalIron _as_bp_third_person_character_2 0)
    (Variables|/Game/ThirdPerson/Blueprints/BP_ThirdPersonCharacter.BP_ThirdPersonCharacter_C|SetPortalEHoney _as_bp_third_person_character_2 0)
    (Variables|/Game/ThirdPerson/Blueprints/BP_ThirdPersonCharacter.BP_ThirdPersonCharacter_C|SetPortalText _as_bp_third_person_character_2 "Максимальный уровень")
    (else
      (Variables|/Game/ThirdPerson/Blueprints/BP_ThirdPersonCharacter.BP_ThirdPersonCharacter_C|SetPortalStone _as_bp_third_person_character 15)
      (Variables|/Game/ThirdPerson/Blueprints/BP_ThirdPersonCharacter.BP_ThirdPersonCharacter_C|SetPortalWood _as_bp_third_person_character 15)
      (Variables|/Game/ThirdPerson/Blueprints/BP_ThirdPersonCharacter.BP_ThirdPersonCharacter_C|SetPortalIron _as_bp_third_person_character 10)
      (Variables|/Game/ThirdPerson/Blueprints/BP_ThirdPersonCharacter.BP_ThirdPersonCharacter_C|SetPortalEHoney _as_bp_third_person_character 5)
      (Variables|/Game/ThirdPerson/Blueprints/BP_ThirdPersonCharacter.BP_ThirdPersonCharacter_C|SetPortalText _as_bp_third_person_character "Улучшить?"))))

(fn ConstructionScript)