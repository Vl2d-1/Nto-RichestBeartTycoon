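; Actor component that makes its owner interactable, giving it a trace target and a screen-space prompt.
; On BeginPlay it adds a box that blocks only GameTraceChannel1, plus a hidden widget component.
; A chain of boolean flags picks the prompt widget for mines, apiaries, fabric, woodcutter and tablets, with a generic fallback.
; ShowInteractionWidget toggles the prompt, and OnInterected calls CallOnInterected.
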(event EventBeginPlay
  (Variables|Default|SetOwner (Components|GetOwner))
  (CallFunction|AddInteractionBox)
  (CallFunction|AddWidget))

(event EventTick
  (params (DeltaSeconds :type Float%20%28single-precision%29)))

(fn AddInteractionBox
  (bind _returnvalue (Game|AddComponentbyClass (Variables|Default|GetOwner) "/Script/Engine.BoxComponent" false))
  (Variables|Default|SetBoxCollision _returnvalue)
  (Components|Box|SetBoxExtent _returnvalue (Variables|Default|GetExtents) true)
  (Collision|SetCollisionResponsetoAllChannels (Variables|Default|GetBoxCollision) "ECR_Ignore")
  (Collision|SetCollisionResponsetoChannel (Variables|Default|GetBoxCollision) "ECC_GameTraceChannel1" "ECR_Block"))

(fn ShowInteractionWidget
  (params (Show? :type Boolean))
  (Rendering|SetVisibility (Variables|Default|GetInteractionWidget) Show? false))

(fn AddWidget
  (if (Variables|Default|GetMine)
    (bind _returnvalue (Game|AddComponentbyClass (Variables|Default|GetOwner) "/Script/UMG.WidgetComponent" false))
    (Transformation|SetRelativeLocation _returnvalue (Variables|Default|GetInteractionWidgetLocation) false false)
    (Class|WidgetComponent|SetWidgetSpace _returnvalue "Screen")
    (Rendering|SetVisibility _returnvalue false false)
    (bind _output_get (Variables|Default|SetInteractionWidget _returnvalue))
    (bind _returnvalue_2 (UserInterface|CreateWidget "/Game/Interaction/InteractionHome/WB_InteractionWidgetMine.WB_InteractionWidgetMine_C" 0 (Variables|Default|GetInteractionName) (Variables|Default|GetStoneInt) (Variables|Default|GetIronInt)))
    (UserInterface|SetWidget _output_get _returnvalue_2)
    (elif (Variables|Default|GetWidgetMine)
      (bind _returnvalue_3 (Game|AddComponentbyClass (Variables|Default|GetOwner) "/Script/UMG.WidgetComponent" false))
      (Transformation|SetRelativeLocation _returnvalue_3 (Variables|Default|GetInteractionWidgetLocation) false false)
      (Class|WidgetComponent|SetWidgetSpace _returnvalue_3 "Screen")
      (Rendering|SetVisibility _returnvalue_3 false false)
      (bind _output_get_2 (Variables|Default|SetInteractionWidget _returnvalue_3))
      (bind _returnvalue_4 (UserInterface|CreateWidget "/Game/Interaction/InteractionHome/WB_InteractionWidgetTabletMine.WB_InteractionWidgetTabletMine_C" 0 (Variables|Default|GetInteractionName) (Variables|Default|GetStoneInt) (Variables|Default|GetWoodInt)))
      (UserInterface|SetWidget _output_get_2 _returnvalue_4)
      (elif (Variables|Default|GetWidgetPortalTablet)
        (bind _returnvalue_5 (Game|AddComponentbyClass (Variables|Default|GetOwner) "/Script/UMG.WidgetComponent" false))
        (Transformation|SetRelativeLocation _returnvalue_5 (Variables|Default|GetInteractionWidgetLocation) false false)
        (Class|WidgetComponent|SetWidgetSpace _returnvalue_5 "Screen")
        (Rendering|SetVisibility _returnvalue_5 false false)
        (bind _output_get_3 (Variables|Default|SetInteractionWidget _returnvalue_5))
        (bind _returnvalue_6 (UserInterface|CreateWidget "/Game/Interaction/InteractionHome/WB_InteractionWidgetTabletPortal.WB_InteractionWidgetTabletPortal_C"))
        (UserInterface|SetWidget _output_get_3 _returnvalue_6)
        (elif (Variables|Default|GetWidgetApiaryTablet)
          (bind _returnvalue_7 (Game|AddComponentbyClass (Variables|Default|GetOwner) "/Script/UMG.WidgetComponent" false))
          (Transformation|SetRelativeLocation _returnvalue_7 (Variables|Default|GetInteractionWidgetLocation) false false)
          (Class|WidgetComponent|SetWidgetSpace _returnvalue_7 "Screen")
          (Rendering|SetVisibility _returnvalue_7 false false)
          (bind _output_get_4 (Variables|Default|SetInteractionWidget _returnvalue_7))
          (bind _returnvalue_8 (UserInterface|CreateWidget "/Game/Interaction/InteractionHome/WB_InteractionWidgetTabletApiary.WB_InteractionWidgetTabletApiary_C"))
          (UserInterface|SetWidget _output_get_4 _returnvalue_8)
          (elif (Variables|Default|GetApiary)
            (bind _returnvalue_9 (Game|AddComponentbyClass (Variables|Default|GetOwner) "/Script/UMG.WidgetComponent" false))
            (Transformation|SetRelativeLocation _returnvalue_9 (Variables|Default|GetInteractionWidgetLocation) false false)
            (Class|WidgetComponent|SetWidgetSpace _returnvalue_9 "Screen")
            (Rendering|SetVisibility _returnvalue_9 false false)
            (bind _output_get_5 (Variables|Default|SetInteractionWidget _returnvalue_9))
            (bind _returnvalue_10 (UserInterface|CreateWidget "/Game/Interaction/InteractionHome/WB_InteractionWidgetApiary.WB_InteractionWidgetApiary_C" 0 (Variables|Default|GetInteractionName)))
            (UserInterface|SetWidget _output_get_5 _returnvalue_10)
            (elif (Variables|Default|GetFabricHoney)
              (bind _returnvalue_11 (Game|AddComponentbyClass (Variables|Default|GetOwner) "/Script/UMG.WidgetComponent" false))
              (Transformation|SetRelativeLocation _returnvalue_11 (Variables|Default|GetInteractionWidgetLocation) false false)
              (Class|WidgetComponent|SetWidgetSpace _returnvalue_11 "Screen")
              (Rendering|SetVisibility _returnvalue_11 false false)
              (bind _output_get_6 (Variables|Default|SetInteractionWidget _returnvalue_11))
              (bind _returnvalue_12 (UserInterface|CreateWidget "/Game/Interaction/InteractionHome/WB_InteractionWidgetFabric1.WB_InteractionWidgetFabric1_C"))
              (UserInterface|SetWidget _output_get_6 _returnvalue_12)
              (elif (Variables|Default|GetFanricEHoney)
                (bind _returnvalue_13 (Game|AddComponentbyClass (Variables|Default|GetOwner) "/Script/UMG.WidgetComponent" false))
                (Transformation|SetRelativeLocation _returnvalue_13 (Variables|Default|GetInteractionWidgetLocation) false false)
                (Class|WidgetComponent|SetWidgetSpace _returnvalue_13 "Screen")
                (Rendering|SetVisibility _returnvalue_13 false false)
                (bind _output_get_7 (Variables|Default|SetInteractionWidget _returnvalue_13))
                (bind _returnvalue_14 (UserInterface|CreateWidget "/Game/Interaction/InteractionHome/WB_InteractionWidgetFabric2.WB_InteractionWidgetFabric2_C"))
                (UserInterface|SetWidget _output_get_7 _returnvalue_14)
                (elif (Variables|Default|GetWoodCutter)
                  (bind _returnvalue_15 (Game|AddComponentbyClass (Variables|Default|GetOwner) "/Script/UMG.WidgetComponent" false))
                  (Transformation|SetRelativeLocation _returnvalue_15 (Variables|Default|GetInteractionWidgetLocation) false false)
                  (Class|WidgetComponent|SetWidgetSpace _returnvalue_15 "Screen")
                  (Rendering|SetVisibility _returnvalue_15 false false)
                  (bind _output_get_8 (Variables|Default|SetInteractionWidget _returnvalue_15))
                  (bind _returnvalue_16 (UserInterface|CreateWidget "/Game/Interaction/InteractionHome/WB_InteractionWidgetWood.WB_InteractionWidgetWood_C"))
                  (UserInterface|SetWidget _output_get_8 _returnvalue_16)
                  (elif (Variables|Default|GetTabletWood)
                    (bind _returnvalue_17 (Game|AddComponentbyClass (Variables|Default|GetOwner) "/Script/UMG.WidgetComponent" false))
                    (Transformation|SetRelativeLocation _returnvalue_17 (Variables|Default|GetInteractionWidgetLocation) false false)
                    (Class|WidgetComponent|SetWidgetSpace _returnvalue_17 "Screen")
                    (Rendering|SetVisibility _returnvalue_17 false false)
                    (bind _output_get_9 (Variables|Default|SetInteractionWidget _returnvalue_17))
                    (bind _returnvalue_18 (UserInterface|CreateWidget "/Game/Interaction/InteractionHome/WB_InteractionWidgetTabletWood.WB_InteractionWidgetTabletWood_C"))
                    (UserInterface|SetWidget _output_get_9 _returnvalue_18)
                    (else
                      (bind _returnvalue_19 (Game|AddComponentbyClass (Variables|Default|GetOwner) "/Script/UMG.WidgetComponent" false))
                      (Transformation|SetRelativeLocation _returnvalue_19 (Variables|Default|GetInteractionWidgetLocation) false false)
                      (Class|WidgetComponent|SetWidgetSpace _returnvalue_19 "Screen")
                      (Rendering|SetVisibility _returnvalue_19 false false)
                      (bind _output_get_10 (Variables|Default|SetInteractionWidget _returnvalue_19))
                      (bind _returnvalue_20 (UserInterface|CreateWidget "/Game/Interaction/WB_InteractionWidget.WB_InteractionWidget_C" 0 (Variables|Default|GetInteractionName)))
                      (UserInterface|SetWidget _output_get_10 _returnvalue_20))))))))))))

(fn OnInterected
  (Default|CallOnInterected))